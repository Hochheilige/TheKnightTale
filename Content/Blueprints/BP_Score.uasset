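; BP_Score is a score table actor that displays a BP_ScoreWidget through its Widget component.
; On BeginPlay it casts and caches that widget in ScoreWidget.
; MoveScoreTable waits one second, then teleports the actor to the opposite side of the world origin by negating X and Y and turning yaw 180 degrees.
; The Set function is an empty stub.
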(event `self.ReceiveBeginPlay`
  (bind _asbp_score_widget (cast `/Game/Blueprints/BP_ScoreWidget` (`WidgetComponent.GetWidget` (`self.Widget`))))
  (set `self.ScoreWidget` _asbp_score_widget))

(event `MoveScoreTable`
  (bind _defaultsceneroot (`self.DefaultSceneRoot`))
  (bind (_returnvalue_x _returnvalue_y _returnvalue_z) (`KismetMathLibrary.BreakVector` (`SceneComponent.K2_GetComponentLocation` _defaultsceneroot)))
  (bind (_returnvalue_roll _returnvalue_pitch _returnvalue_yaw) (`KismetMathLibrary.BreakRotator` (`SceneComponent.K2_GetComponentRotation` _defaultsceneroot)))
  (`KismetSystemLibrary.Delay` 1.0)
  (`self.K2_SetActorLocationAndRotation` (`KismetMathLibrary.MakeVector` (* -1 _returnvalue_x) (* -1 _returnvalue_y) _returnvalue_z) (`KismetMathLibrary.MakeRotator` _returnvalue_roll _returnvalue_pitch (- _returnvalue_yaw 180.0)) false true))

(fn `Set`)

(fn `UserConstructionScript`)