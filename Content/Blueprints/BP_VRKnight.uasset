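; VR knight pawn that rides a horse along a Trajectory spline and breaks its spear on contact.
; StartBattle_1 enables Tick-driven distance movement with adjustable Speed, while StartBattle plays a HorseMover timeline with input-adjusted Duration controlling play rate.
; Spear overlap spawns particles, disables collision and shows a broken spear and text, then restores after a delay.
; Axis-based movement is also wired but noted as faulty.
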(event `self.ReceiveBeginPlay`
  ;[0.03434 0.03434 0.03434] Begin Play - Set Tracking Origin to eye level
  (if (`HeadMountedDisplayFunctionLibrary.IsHeadMountedDisplayEnabled`)
    (`HeadMountedDisplayFunctionLibrary.SetTrackingOrigin` "Eye")))

(event `self.ReceiveTick`
  (params (DeltaSeconds :type "Float (single-precision)"))
  (if (`self.IsBattleBegin`)
    (`self.MoveHorseSpline`)
    (add `self.IncreaseSpeed` (delegate `IncreaseSpeedEvent`))))

(event `IncreaseSpeedEvent`
  (set `self.Speed` (+ (`self.Speed`) 1.0)))

(event `InputAction|StartBattle_1`
  (params (Key :type "Key Structure"))
  (:`Pressed`
    (set `self.IsBattleBegin` true)))

(event `InputAction|IncreaseSpeed`
  (params (Key :type "Key Structure"))
  (:`Pressed`
    (`self.IncreaseSpeedEvent`)))

(event `InputAction|IncreaseSpeed`
  (params (Key :type "Key Structure"))
  ;[1 1 1] Increase/Reduce speed
  (:`Pressed`
    (set `self.Duration` (- (`self.Duration`) 1.0))))

(event `MoveHorseTimerSpline`
  (bind _returnvalue (`KismetMathLibrary.Lerp` 0.0 (`SplineComponent.GetSplineLength` (`/Game/Blueprints/BP_Trajectory.Trajectory` (`self.Trajectory`))) (`self.Alpha`)))
  (`TimelineComponent.SetPlayRate` (`self.HorseMover`) (/ 1.0 (`self.Duration`)))
  (`TimelineComponent.SetNewTime` (`self.HorseMover`) 0.0)
  (bind (_direction _alpha) (`Timeline|HorseMover`)
    (:`Update`
      (set `self.Alpha` _alpha)
      (`TimelineComponent.SetPlayRate` (`self.HorseMover`) (/ 1.0 (`self.Duration`)))
      (`self.K2_SetActorLocationAndRotation` (`SplineComponent.GetLocationAtDistanceAlongSpline` (`/Game/Blueprints/BP_Trajectory.Trajectory` (`self.Trajectory`)) _returnvalue "World") (`SplineComponent.GetRotationAtDistanceAlongSpline` (`/Game/Blueprints/BP_Trajectory.Trajectory` (`self.Trajectory`)) _returnvalue "World")))))

(event `InputAction|ReduceSpeed`
  (params (Key :type "Key Structure"))
  ;[1 1 1] Increase/Reduce speed
  (:`Pressed`
    (set `self.Duration` (+ (`self.Duration`) 1.0))))

(event `MoveHorseSpline`
  (bind _distance (`self.Distance`))
  (bind _trajectory (`/Game/Blueprints/BP_Trajectory.Trajectory` (`self.Trajectory`)))
  (set `self.Distance` (+ (`self.Distance`) (`self.Speed`)))
  (`self.K2_SetActorLocationAndRotation` (`SplineComponent.GetLocationAtDistanceAlongSpline` _trajectory _distance "World") (`SplineComponent.GetRotationAtDistanceAlongSpline` _trajectory _distance "World") true))

(event `InputAxis|MoveForward` :overrideparent false
  (params (AxisValue :type "Float (single-precision)"))
  ;[1 1 1] Moving but work dont quite right
  (if (not (== AxisValue 0.0))
    (`self.AddMovementInput` (`SceneComponent.GetForwardVector` (`self.Arrow`)) (* AxisValue (`self.MovementSpeed`)))))

(event `InputAxis|MoveBackward`
  (params (AxisValue :type "Float (single-precision)"))
  ;[1 1 1] Moving but work dont quite right
  (if (not (== AxisValue 0.0))
    (`self.AddMovementInput` (`SceneComponent.GetForwardVector` (`self.Arrow`)) (* AxisValue (`self.MovementSpeed`)))))

(event `self.SpearCollision.OnComponentBeginOverlap`
  (params (OverlappedComponent :type "PrimitiveComponent Object Reference") (OtherActor :type "Actor Object Reference") (OtherComp :type "PrimitiveComponent Object Reference") (OtherBodyIndex :type Integer) (bFromSweep :type Boolean) (SweepResult :type "HitResult Structure (by ref)"))
  (`self.SetSpearCollision`)
  (`AddComponent|NODE_AddParticleSystemComponent-0` :`RelativeTransform` (`KismetMathLibrary.MakeRelativeTransform` (`SceneComponent.K2_GetComponentToWorld` (`self.SpearCollision`)) (`SceneComponent.K2_GetComponentToWorld` (`self.DefaultSceneRoot`))))
  (`self.SetSpearVisibility`)
  (`KismetSystemLibrary.Delay` 3.0)
  (`self.SetSpearVisibility`)
  (`self.SetSpearCollision`))

(event `InputAxis|MoveLeft`
  (params (AxisValue :type "Float (single-precision)"))
  ;[1 1 1] Moving but work dont quite right
  (if (not (== AxisValue 0.0))
    (`self.AddMovementInput` (`SceneComponent.GetRightVector` (`self.Arrow`)) (* AxisValue (`self.MovementSpeed`)))))

(event `InputAxis|MoveRight`
  (params (AxisValue :type "Float (single-precision)"))
  ;[1 1 1] Moving but work dont quite right
  (if (not (== AxisValue 0.0))
    (`self.AddMovementInput` (`SceneComponent.GetRightVector` (`self.Arrow`)) (* AxisValue (`self.MovementSpeed`)))))

(event `InputAction|StartBattle`
  (params (Key :type "Key Structure"))
  (:`Pressed`
    (`self.MoveHorseTimerSpline`)))

(fn `SetSpearCollision`
  (if (`self.IsCollisionEnable`)
    (`PrimitiveComponent.SetCollisionEnabled` (`self.SpearCollision`) "NoCollision")
    (set `self.IsCollisionEnable` false)
    (else
      (`PrimitiveComponent.SetCollisionEnabled` (`self.SpearCollision`) "QueryAndPhysics")
      (set `self.IsCollisionEnable` true))))

(fn `SetSpearVisibility`
  (if (`self.IsVisible`)
    (`SceneComponent.SetVisibility` (`self.Spear`) false false)
    (`SceneComponent.SetVisibility` (`self.BrokenSpear`) true false)
    (`SceneComponent.SetVisibility` (`self.TextRender`) true false)
    (set `self.IsVisible` false)
    (else
      (`SceneComponent.SetVisibility` (`self.TextRender`) false false)
      (`SceneComponent.SetVisibility` (`self.Spear`) true false)
      (`SceneComponent.SetVisibility` (`self.BrokenSpear`) false false)
      (set `self.IsVisible` true))))

(fn `UserConstructionScript`)