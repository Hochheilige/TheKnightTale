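; Game mode for a VR knight game that scores hits on a mannequin and triggers movement of the mannequin and score table.
; Construction caches the score actor, knight and mannequin via actor lookups.
; UpdateScore uses the current score to pick score images, turning them green for body (+1) or head (+2) hits.
; Horse hits subtract three and turn all three images red; the score-three branch has no wired outcomes.
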(event `MoveObjectsOnScene`
  (`/Game/Blueprints/BP_Manequen.MoveManequen` (`self.Manequen`))
  (`/Game/Blueprints/BP_Score.MoveScoreTable` (`self.ScoreWidget`)))

(event `UpdateScore`
  (params (ManequenPart :type "/Game/Blueprints/ScoreEnum Enum" :default "NewEnumerator0"))
  (bind _score_2 (`/Game/Blueprints/BP_ScoreWidget.Score_2` (`/Game/Blueprints/BP_Score.ScoreWidget` (`self.ScoreWidget`))))
  (bind _score_3 (`/Game/Blueprints/BP_ScoreWidget.Score_3` (`/Game/Blueprints/BP_Score.ScoreWidget` (`self.ScoreWidget`))))
  (if (`self.IsScoreEmpty`)
    (`self.SetScoreOnTable` ManequenPart (`/Game/Blueprints/BP_ScoreWidget.Score_1` (`/Game/Blueprints/BP_Score.ScoreWidget` (`self.ScoreWidget`))) _score_2)
    (elif (`self.IsScoreOne`)
      (`self.SetScoreOnTable` ManequenPart _score_2 _score_3)
      (elif (`self.IsScoreTwo`)
        (`self.SetScoreOnTable` ManequenPart _score_3 _score_3)
        (elif (`self.IsScoreThree`)
          (switch `/Game/Blueprints/ScoreEnum` ManequenPart))))))

(fn `IncreaseScore`
  (set `self.CharacterScore` (+ (`self.CharacterScore`) 1)))

(fn `IsAllScoreColorSet`
  (params (ColorToCheck :type "LinearColor Structure"))
  (returns (IsAllScoreColorSet :type Boolean))
  (bind _scorewidget (`/Game/Blueprints/BP_Score.ScoreWidget` (`self.ScoreWidget`)))
  (return (== (== (`self.IsScoreColorSet` (`/Game/Blueprints/BP_ScoreWidget.Score_1` _scorewidget) ColorToCheck) (`self.IsScoreColorSet` (`/Game/Blueprints/BP_ScoreWidget.Score_2` _scorewidget) ColorToCheck)) (`self.IsScoreColorSet` (`/Game/Blueprints/BP_ScoreWidget.Score_3` _scorewidget) ColorToCheck))))

(fn `IsScoreColorSet`
  (params (ScoreImage :type "Image Object Reference") (ColorToCheck :type "LinearColor Structure"))
  (returns (IsScoreColorSet :type Boolean))
  (return (== (`Image.ColorAndOpacity` ScoreImage) ColorToCheck)))

(fn `IsScoreEmpty`
  (returns (IsScoreEmpty :type Boolean))
  (return (== (`self.CharacterScore`) 0)))

(fn `IsScoreOne`
  (returns (IsScoreOne :type Boolean))
  (return (== (`self.CharacterScore`) 1)))

(fn `IsScoreThree`
  (returns (IsScoreThree :type Boolean))
  (return (== (`self.CharacterScore`) 3)))

(fn `IsScoreTwo`
  (returns (IsScoreTwo :type Boolean))
  (return (== (`self.CharacterScore`) 2)))

(fn `Set Score For Body Hit`
  (params (ScoreImage :type "Image Object Reference"))
  (set `self.CharacterScore` (+ (`self.CharacterScore`) 1))
  (`Image.SetColorAndOpacity` ScoreImage (struct :`G` 1.0 :`A` 1.0)))

(fn `SetScoreForHeadHit`
  (params (ScoreImage0 :type "Image Object Reference") (ScoreImage1 :type "Image Object Reference"))
  (set `self.CharacterScore` (+ 2 (`self.CharacterScore`)))
  (`Image.SetColorAndOpacity` ScoreImage0 (struct :`G` 1.0 :`A` 1.0))
  (`Image.SetColorAndOpacity` ScoreImage1 (struct :`G` 1.0 :`A` 1.0)))

(fn `SetScoreForHorseHit`
  (set `self.CharacterScore` (- (`self.CharacterScore`) 3))
  (`self.UpdateScoreColor` (struct :`R` 1.0 :`A` 1.0)))

(fn `SetScoreOnTable`
  (params (HitPlace :type "/Game/Blueprints/ScoreEnum Enum" :default "NewEnumerator1") (ScoreImage0 :type "Image Object Reference") (ScoreImage1 :type "Image Object Reference"))
  (switch `/Game/Blueprints/ScoreEnum` HitPlace
    (:`NewEnumerator1`
      (`self.Set Score For Body Hit` ScoreImage0))
    (:`NewEnumerator0`
      (`self.SetScoreForHeadHit` ScoreImage0 ScoreImage1))
    (:`NewEnumerator3`
      (`self.SetScoreForHorseHit`))))

(fn `UpdateScoreColor`
  (params (NewColor :type "LinearColor Structure"))
  (bind _scorewidget (`/Game/Blueprints/BP_Score.ScoreWidget` (`self.ScoreWidget`)))
  (`|ExecutionSequence`
    (:`then_0`
      (`Image.SetColorAndOpacity` (`/Game/Blueprints/BP_ScoreWidget.Score_1` _scorewidget) NewColor))
    (:`then_1`
      (`Image.SetColorAndOpacity` (`/Game/Blueprints/BP_ScoreWidget.Score_2` _scorewidget) NewColor))
    (:`then_2`
      (`Image.SetColorAndOpacity` (`/Game/Blueprints/BP_ScoreWidget.Score_3` _scorewidget) NewColor))))

(fn `UserConstructionScript`
  (`|ExecutionSequence`
    (:`then_0`
      (bind _returnvalue (`GameplayStatics.GetActorOfClass` "/Game/Blueprints/BP_Score.BP_Score_C"))
      (set `self.ScoreWidget` _returnvalue)
      (set `self.CharacterScore` 0))
    (:`then_1`
      (bind _returnvalue_2 (`GameplayStatics.GetActorOfClass` "/Game/Blueprints/BP_VRKnight.BP_VRKnight_C"))
      (set `self.Character` _returnvalue_2))
    (:`then_2`
      (bind _returnvalue_3 (`GameplayStatics.GetActorOfClass` "/Game/Blueprints/BP_Manequen.BP_Manequen_C"))
      (set `self.Manequen` _returnvalue_3))))