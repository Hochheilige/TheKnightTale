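; Mounted mannequin target with shield, horse, head and body hit zones; all but the shield update the player's score through BP_Gamemode.
; Head or body hits toggle that part's physics and the other zones' collision, then toggle the struck part's physics and collision after a delay.
; Every hit ends with a delayed MoveObjectsOnScene call on the game mode.
; GetNewTransform provides an X/Y-mirrored, yaw-flipped transform; BeginPlay sets head, body and horse to ignore each other when moving.
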(event `self.ReceiveBeginPlay`
  (`self.IgnoreComponentsWhenMoving`))

(event `self.ShieldCollision.OnComponentBeginOverlap`
  (params (OverlappedComponent :type "PrimitiveComponent Object Reference") (OtherActor :type "Actor Object Reference") (OtherComp :type "PrimitiveComponent Object Reference") (OtherBodyIndex :type Integer) (bFromSweep :type Boolean) (SweepResult :type "HitResult Structure (by ref)"))
  ;[1 1 1] Collisions
  (`KismetSystemLibrary.PrintString` "Hit to Shield")
  (bind _asbp_gamemode (cast `/Game/Blueprints/BP_Gamemode` (`GameplayStatics.GetGameMode`)))
  (`KismetSystemLibrary.Delay` 3.0)
  (`/Game/Blueprints/BP_Gamemode.MoveObjectsOnScene` _asbp_gamemode))

(event `self.HorseCollision.OnComponentBeginOverlap`
  (params (OverlappedComponent :type "PrimitiveComponent Object Reference") (OtherActor :type "Actor Object Reference") (OtherComp :type "PrimitiveComponent Object Reference") (OtherBodyIndex :type Integer) (bFromSweep :type Boolean) (SweepResult :type "HitResult Structure (by ref)"))
  ;[1 1 1] Collisions
  (`KismetSystemLibrary.PrintString` "Hit to Horse")
  (bind _asbp_gamemode (cast `/Game/Blueprints/BP_Gamemode` (`GameplayStatics.GetGameMode`)))
  (`/Game/Blueprints/BP_Gamemode.UpdatePlayerScore` _asbp_gamemode "NewEnumerator3")
  (`KismetSystemLibrary.Delay` 3.0)
  (`/Game/Blueprints/BP_Gamemode.MoveObjectsOnScene` _asbp_gamemode))

(event `self.HeadCollision.OnComponentBeginOverlap`
  (params (OverlappedComponent :type "PrimitiveComponent Object Reference") (OtherActor :type "Actor Object Reference") (OtherComp :type "PrimitiveComponent Object Reference") (OtherBodyIndex :type Integer) (bFromSweep :type Boolean) (SweepResult :type "HitResult Structure (by ref)"))
  ;[1 1 1] Collisions
  (`KismetSystemLibrary.PrintString` "Hit to Head")
  (`|ExecutionSequence`
    (:`then_0`
      (`self.UpdateHorseCollision`)
      (`self.UpdateBodyCollision`)
      (`self.UpdateHeadPhysics`))
    (:`then_1`
      (bind _asbp_gamemode (cast `/Game/Blueprints/BP_Gamemode` (`GameplayStatics.GetGameMode`)))
      (`/Game/Blueprints/BP_Gamemode.UpdatePlayerScore` _asbp_gamemode "NewEnumerator0")
      (`KismetSystemLibrary.Delay` 3.0)
      (`self.UpdateHeadState`)
      (`/Game/Blueprints/BP_Gamemode.MoveObjectsOnScene` _asbp_gamemode))))

(event `self.BodyCollision.OnComponentBeginOverlap`
  (params (OverlappedComponent :type "PrimitiveComponent Object Reference") (OtherActor :type "Actor Object Reference") (OtherComp :type "PrimitiveComponent Object Reference") (OtherBodyIndex :type Integer) (bFromSweep :type Boolean) (SweepResult :type "HitResult Structure (by ref)"))
  ;[1 1 1] Collisions
  (`KismetSystemLibrary.PrintString` "Hit to Body")
  (`|ExecutionSequence`
    (:`then_0`
      (`self.UpdateHorseCollision`)
      (`self.UpdateHeadCollision`)
      (`self.UpdateBodyPhysics`))
    (:`then_1`
      (bind _asbp_gamemode (cast `/Game/Blueprints/BP_Gamemode` (`GameplayStatics.GetGameMode`)))
      (`/Game/Blueprints/BP_Gamemode.UpdatePlayerScore` _asbp_gamemode "NewEnumerator1")
      (`KismetSystemLibrary.Delay` 3.0)
      (`self.UpdateBodyState`)
      (`/Game/Blueprints/BP_Gamemode.MoveObjectsOnScene` _asbp_gamemode))))

(fn `GetNewTransform`
  (returns (ResTransform :type "Transform Structure"))
  (return (`KismetMathLibrary.MakeTransform` (`KismetMathLibrary.MakeVector` (* -1 (.x (.location (`self.GetTransform`)))) (* -1 (.y (.location (`self.GetTransform`)))) (.z (.location (`self.GetTransform`)))) (`KismetMathLibrary.MakeRotator` (.roll (.rotation (`self.GetTransform`))) (.pitch (.rotation (`self.GetTransform`))) (- (.yaw (.rotation (`self.GetTransform`))) 180.0)) (.scale (`self.GetTransform`)))))

(fn `IgnoreComponentsWhenMoving`
  (`|ExecutionSequence`
    (:`then_0`
      (`PrimitiveComponent.IgnoreComponentWhenMoving` (`self.HeadCollision`) (`self.Body`) true)
      (`PrimitiveComponent.IgnoreComponentWhenMoving` (`self.Head`) (`self.Body`) true)
      (`PrimitiveComponent.IgnoreComponentWhenMoving` (`self.HeadCollision`) (`self.BodyCollision`) true)
      (`PrimitiveComponent.IgnoreComponentWhenMoving` (`self.Head`) (`self.BodyCollision`) true))
    (:`then_1`
      (`PrimitiveComponent.IgnoreComponentWhenMoving` (`self.BodyCollision`) (`self.Head`) true)
      (`PrimitiveComponent.IgnoreComponentWhenMoving` (`self.BodyCollision`) (`self.HeadCollision`) true)
      (`PrimitiveComponent.IgnoreComponentWhenMoving` (`self.Body`) (`self.Head`) true)
      (`PrimitiveComponent.IgnoreComponentWhenMoving` (`self.Body`) (`self.HeadCollision`) true))
    (:`then_2`
      (`PrimitiveComponent.IgnoreComponentWhenMoving` (`self.BodyCollision`) (`self.Horse`) true)
      (`PrimitiveComponent.IgnoreComponentWhenMoving` (`self.BodyCollision`) (`self.HorseCollision`) true)
      (`PrimitiveComponent.IgnoreComponentWhenMoving` (`self.Body`) (`self.Horse`) true)
      (`PrimitiveComponent.IgnoreComponentWhenMoving` (`self.Body`) (`self.HorseCollision`) true))
    (:`then_3`
      (`PrimitiveComponent.IgnoreComponentWhenMoving` (`self.Horse`) (`self.BodyCollision`) true)
      (`PrimitiveComponent.IgnoreComponentWhenMoving` (`self.HorseCollision`) (`self.BodyCollision`) true)
      (`PrimitiveComponent.IgnoreComponentWhenMoving` (`self.Horse`) (`self.Body`) true)
      (`PrimitiveComponent.IgnoreComponentWhenMoving` (`self.HorseCollision`) (`self.Body`) true))
    (:`then_4`
      (`PrimitiveComponent.IgnoreComponentWhenMoving` (`self.HeadCollision`) (`self.Horse`) true)
      (`PrimitiveComponent.IgnoreComponentWhenMoving` (`self.HeadCollision`) (`self.HorseCollision`) true)
      (`PrimitiveComponent.IgnoreComponentWhenMoving` (`self.Head`) (`self.Horse`) true)
      (`PrimitiveComponent.IgnoreComponentWhenMoving` (`self.Head`) (`self.HorseCollision`) true))
    (:`then_5`
      (`PrimitiveComponent.IgnoreComponentWhenMoving` (`self.Horse`) (`self.HeadCollision`) true)
      (`PrimitiveComponent.IgnoreComponentWhenMoving` (`self.HorseCollision`) (`self.HeadCollision`) true)
      (`PrimitiveComponent.IgnoreComponentWhenMoving` (`self.Horse`) (`self.HeadCollision`) true)
      (`PrimitiveComponent.IgnoreComponentWhenMoving` (`self.HorseCollision`) (`self.Head`) true))))

(fn `UpdateBodyCollision`
  (if (`PrimitiveComponent.K2_IsCollisionEnabled` (`self.Body`))
    (`PrimitiveComponent.SetCollisionEnabled` (`self.Body`) "NoCollision")
    (`PrimitiveComponent.SetCollisionEnabled` (`self.BodyCollision`) "NoCollision")
    (else
      (`PrimitiveComponent.SetCollisionEnabled` (`self.Body`) "PhysicsOnly")
      (`PrimitiveComponent.SetCollisionEnabled` (`self.BodyCollision`) "QueryOnly"))))

(fn `UpdateBodyPhysics`
  (if (`SceneComponent.IsSimulatingPhysics` (`self.Body`) "None")
    (`PrimitiveComponent.SetSimulatePhysics` (`self.Body`) false)
    (else
      (`PrimitiveComponent.SetSimulatePhysics` (`self.Body`) true))))

(fn `UpdateBodyState`
  (`|ExecutionSequence`
    (:`then_0`
      (`self.UpdateBodyPhysics`))
    (:`then_1`
      (`self.UpdateBodyCollision`))))

(fn `UpdateHeadCollision`
  (if (`PrimitiveComponent.K2_IsCollisionEnabled` (`self.Head`))
    (`PrimitiveComponent.SetCollisionEnabled` (`self.Head`) "NoCollision")
    (`PrimitiveComponent.SetCollisionEnabled` (`self.HeadCollision`) "NoCollision")
    (else
      (`PrimitiveComponent.SetCollisionEnabled` (`self.Head`) "PhysicsOnly")
      (`PrimitiveComponent.SetCollisionEnabled` (`self.HeadCollision`) "QueryOnly"))))

(fn `UpdateHeadPhysics`
  (if (`SceneComponent.IsSimulatingPhysics` (`self.Head`) "None")
    (`PrimitiveComponent.SetSimulatePhysics` (`self.Head`) false)
    (else
      (`PrimitiveComponent.SetSimulatePhysics` (`self.Head`) true))))

(fn `UpdateHeadState`
  (`|ExecutionSequence`
    (:`then_0`
      (`self.UpdateHeadPhysics`))
    (:`then_1`
      (`self.UpdateHeadCollision`))))

(fn `UpdateHorseCollision`
  (if (`PrimitiveComponent.K2_IsCollisionEnabled` (`self.Horse`))
    (`PrimitiveComponent.SetCollisionEnabled` (`self.Horse`) "NoCollision")
    (`PrimitiveComponent.SetCollisionEnabled` (`self.HorseCollision`) "NoCollision")
    (else
      (`PrimitiveComponent.SetCollisionEnabled` (`self.Horse`) "PhysicsOnly")
      (`PrimitiveComponent.SetCollisionEnabled` (`self.HorseCollision`) "QueryOnly"))))

(fn `UserConstructionScript`)