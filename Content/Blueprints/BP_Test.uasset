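; BP_Test is a test Blueprint that moves its static mesh along the spline of a referenced Trajectory object.
; BeginPlay sets the starting distance, and each Tick advances it by a fixed step, so speed depends on frame rate.
; The mesh moves to the world-space point at that spline distance with sweep enabled, leaving its rotation unchanged.
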(event `self.ReceiveBeginPlay`
  (set `self.Distance` 10.0))

(event `self.ReceiveTick`
  (params (DeltaSeconds :type "Float (single-precision)"))
  (set `self.Distance` (+ (`self.Distance`) 1.0))
  (`SceneComponent.K2_SetWorldLocation` (`self.StaticMesh`) (`SplineComponent.GetLocationAtDistanceAlongSpline` (`/Game/Blueprints/BP_Trajectory.Trajectory` (`self.Trajectory`)) (`self.Distance`) "World") true false))

(fn `UserConstructionScript`)