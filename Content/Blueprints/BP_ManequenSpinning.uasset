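; Spinning mannequin that animates its hands and shield, starting on BeginPlay.
; The HandsRotator timeline pitches the Hands component relative to its captured starting rotation.
; Each of its updates calls MoveShiled, which re-captures the ShieldRotationPoint transform and plays ShieldMoverAndRotator.
; That timeline offsets the shield pivot's location and yaw from the most recently captured values.
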(event `self.ReceiveBeginPlay`
  (`self.IgnoreComponentsWhenMoving`)
  (`self.RotateHands`))

(event `RotateHands`
  ;[1 1 1] Event for rotating manequen hands
  (set `self.StartHandsRotation` (`SceneComponent.RelativeRotation` (`self.Hands`)))
  (bind (_direction _angle) (`Timeline|HandsRotator`)
    (:`Update`
      (`SceneComponent.K2_SetRelativeRotation` (`self.Hands`) (`KismetMathLibrary.ComposeRotators` (`self.StartHandsRotation`) (`KismetMathLibrary.MakeRotator` 0.0 _angle)) false false)
      (`self.MoveShiled`))))

(event `MoveShiled`
  (bind _shieldrotationpoint (`self.ShieldRotationPoint`))
  (set `self.StartShieldLoaction` (`SceneComponent.RelativeLocation` _shieldrotationpoint))
  (set `self.StartShieldRotation` (`SceneComponent.RelativeRotation` _shieldrotationpoint))
  (bind (_direction _location _angle) (`Timeline|ShieldMoverAndRotator`)
    (:`Update`
      (`SceneComponent.K2_SetRelativeLocationAndRotation` (`self.ShieldRotationPoint`) (+ (`self.StartShieldLoaction`) _location) (`KismetMathLibrary.ComposeRotators` (`KismetMathLibrary.MakeRotator` 0.0 0.0 _angle) (`self.StartShieldRotation`)) false false))))

(fn `UserConstructionScript`)