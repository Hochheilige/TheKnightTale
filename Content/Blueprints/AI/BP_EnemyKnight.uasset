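; Mounted enemy knight AI pawn built from body, head, horse, weapon and quiver parts.
; StartRun and StopRun toggle the ReadyToRun blackboard key and a moving flag, starting false.
; Perception updates alternate via IsSaw, firing the attack dispatcher with a brief IsAttack window.
; Body, head and horse overlaps set HitPlace and fire the hit dispatcher; helpers sync animations and stop parts colliding with each other while moving.
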(event `self.ReceiveBeginPlay`
  ;[0 0.6857 1] Враг с начала не готов бежать вперед
  (`BlackboardComponent.SetValueAsBool` (`AIBlueprintHelperLibrary.GetBlackboard` null) "ReadyToRun" false)
  (`self.IgnoreComponentsWhenMoving`))

(event `self.AIPerception.OnPerceptionUpdated`
  (params (UpdatedActors :type "Array of Actor Object Reference (by ref)"))
  (if (`self.IsSaw`)
    (set `self.IsSaw` false)
    (else
      (set `self.IsAttack` true)
      (`KismetSystemLibrary.PrintString` "ATTACK")
      (`self.AttackDispatcher`)
      (`KismetSystemLibrary.Delay` 0.2)
      (set `self.IsAttack` false)
      (set `self.IsSaw` true))))

(event `StartRun`
  ;[0 0.6447 1] Старт забега
  (`BlackboardComponent.SetValueAsBool` (`AIBlueprintHelperLibrary.GetBlackboard` null) "ReadyToRun" true)
  (set `self.IsStartMoving` true)
  (`KismetSystemLibrary.PrintString` "Hello"))

(event `StopRun`
  (`BlackboardComponent.SetValueAsBool` (`AIBlueprintHelperLibrary.GetBlackboard` null) "ReadyToRun" false)
  (set `self.IsStartMoving` false))

(event `self.Body.OnComponentBeginOverlap`
  (params (OverlappedComponent :type "PrimitiveComponent Object Reference") (OtherActor :type "Actor Object Reference") (OtherComp :type "PrimitiveComponent Object Reference") (OtherBodyIndex :type Integer) (bFromSweep :type Boolean) (SweepResult :type "HitResult Structure (by ref)"))
  (set `self.HitPlace` "NewEnumerator1")
  (`self.HitDispatcher`))

(event `self.Horse.OnComponentBeginOverlap`
  (params (OverlappedComponent :type "PrimitiveComponent Object Reference") (OtherActor :type "Actor Object Reference") (OtherComp :type "PrimitiveComponent Object Reference") (OtherBodyIndex :type Integer) (bFromSweep :type Boolean) (SweepResult :type "HitResult Structure (by ref)"))
  (set `self.HitPlace` "NewEnumerator3")
  (`self.HitDispatcher`))

(event `self.Head.OnComponentBeginOverlap`
  (params (OverlappedComponent :type "PrimitiveComponent Object Reference") (OtherActor :type "Actor Object Reference") (OtherComp :type "PrimitiveComponent Object Reference") (OtherBodyIndex :type Integer) (bFromSweep :type Boolean) (SweepResult :type "HitResult Structure (by ref)"))
  (set `self.HitPlace` "NewEnumerator0")
  (`self.HitDispatcher`))

(fn `EnemyPlayAnimation`
  (params (NewAnimToPlay :type "AnimationAsset Object Reference") (bLooping :type Boolean))
  (`|ExecutionSequence`
    (:`then_0`
      (`SkeletalMeshComponent.PlayAnimation` (`self.Body`) NewAnimToPlay bLooping))
    (:`then_1`
      (`SkeletalMeshComponent.PlayAnimation` (`self.Head`) NewAnimToPlay bLooping))
    (:`then_2`
      (`SkeletalMeshComponent.PlayAnimation` (`self.Horse`) NewAnimToPlay bLooping))))

(fn `IgnoreComponentsWhenMoving`
  (`|ExecutionSequence`
    (:`then_0`
      (`PrimitiveComponent.IgnoreComponentWhenMoving` (`self.Body`) (`self.Quiver`) true)
      (`PrimitiveComponent.IgnoreComponentWhenMoving` (`self.Body`) (`self.Head`) true)
      (`PrimitiveComponent.IgnoreComponentWhenMoving` (`self.Body`) (`self.Weapon_R`) true)
      (`PrimitiveComponent.IgnoreComponentWhenMoving` (`self.Body`) (`self.Horse`) true)
      (`PrimitiveComponent.IgnoreComponentWhenMoving` (`self.Body`) (`self.Weapon_L`) true))
    (:`then_1`
      (`PrimitiveComponent.IgnoreComponentWhenMoving` (`self.Weapon_R`) (`self.Body`) true)
      (`PrimitiveComponent.IgnoreComponentWhenMoving` (`self.Weapon_R`) (`self.Horse`) true)
      (`PrimitiveComponent.IgnoreComponentWhenMoving` (`self.Weapon_R`) (`self.Head`) true)
      (`PrimitiveComponent.IgnoreComponentWhenMoving` (`self.Weapon_R`) (`self.Quiver`) true)
      (`PrimitiveComponent.IgnoreComponentWhenMoving` (`self.Weapon_R`) (`self.Weapon_L`) true))
    (:`then_2`
      (`PrimitiveComponent.IgnoreComponentWhenMoving` (`self.Weapon_L`) (`self.Body`) true)
      (`PrimitiveComponent.IgnoreComponentWhenMoving` (`self.Weapon_L`) (`self.Horse`) true)
      (`PrimitiveComponent.IgnoreComponentWhenMoving` (`self.Weapon_L`) (`self.Head`) true)
      (`PrimitiveComponent.IgnoreComponentWhenMoving` (`self.Weapon_L`) (`self.Quiver`) true)
      (`PrimitiveComponent.IgnoreComponentWhenMoving` (`self.Weapon_L`) (`self.Weapon_R`) true))
    (:`then_3`
      (`PrimitiveComponent.IgnoreComponentWhenMoving` (`self.Horse`) (`self.Head`) true)
      (`PrimitiveComponent.IgnoreComponentWhenMoving` (`self.Horse`) (`self.Quiver`) true)
      (`PrimitiveComponent.IgnoreComponentWhenMoving` (`self.Horse`) (`self.Body`) true)
      (`PrimitiveComponent.IgnoreComponentWhenMoving` (`self.Horse`) (`self.Weapon_R`) true)
      (`PrimitiveComponent.IgnoreComponentWhenMoving` (`self.Horse`) (`self.Weapon_L`) true))
    (:`then_4`
      (`PrimitiveComponent.IgnoreComponentWhenMoving` (`self.Head`) (`self.Horse`) true)
      (`PrimitiveComponent.IgnoreComponentWhenMoving` (`self.Head`) (`self.Quiver`) true)
      (`PrimitiveComponent.IgnoreComponentWhenMoving` (`self.Head`) (`self.Body`) true)
      (`PrimitiveComponent.IgnoreComponentWhenMoving` (`self.Head`) (`self.Weapon_R`) true)
      (`PrimitiveComponent.IgnoreComponentWhenMoving` (`self.Head`) (`self.Weapon_L`) true))
    (:`then_5`
      (`PrimitiveComponent.IgnoreComponentWhenMoving` (`self.Quiver`) (`self.Horse`) true)
      (`PrimitiveComponent.IgnoreComponentWhenMoving` (`self.Quiver`) (`self.Body`) true)
      (`PrimitiveComponent.IgnoreComponentWhenMoving` (`self.Quiver`) (`self.Head`) true)
      (`PrimitiveComponent.IgnoreComponentWhenMoving` (`self.Quiver`) (`self.Weapon_R`) true)
      (`PrimitiveComponent.IgnoreComponentWhenMoving` (`self.Quiver`) (`self.Weapon_L`) true))))

(fn `UserConstructionScript`)