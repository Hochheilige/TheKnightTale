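; BP_FPS_LoS is a level design helper actor that tests eye-level line of sight to another selected instance of itself.
; DrawEyeLine runs a Visibility trace between both Eyeline components, draws it for a set duration, and prints clear, the blocking actor, or an invalid-target warning.
; The construction script raises the Eyeline by an offset and toggles between a chosen skeletal mesh and a capsule as the stand-in body.
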(event `DrawEyeLine`
  (if (== (`self.FPS_LoS`) self)
    (`KismetSystemLibrary.PrintString` "Target is self" true true (struct :`R` 1.0 :`A` 1.0))
    (elif (!= (`self.FPS_LoS`) null)
      (bind (_outhit _returnvalue) (`KismetSystemLibrary.LineTraceSingle` :`Start` (`SceneComponent.K2_GetComponentLocation` (`self.Eyeline`)) :`End` (`SceneComponent.K2_GetComponentLocation` (`/Game/LDTK/Blueprints/BP_FPS_LoS.Eyeline` (`self.FPS_LoS`))) :`TraceChannel` "TraceTypeQuery1" :`DrawDebugType` "ForDuration" :`TraceColor` (struct :`G` 1.0 :`B` 0.039678 :`A` 1.0) :`TraceHitColor` (struct :`R` 1.0 :`G` 0.020984 :`A` 1.0) :`DrawTime` (`self.Duration`)))
      (if _returnvalue
        (`KismetSystemLibrary.PrintString` (`KismetStringLibrary.Concat_StrStr` "Line of sight is blocked by: " (`KismetSystemLibrary.GetDisplayName` (`.HitActor` (`GameplayStatics.BreakHitResult` _outhit)))) true true (struct :`G` 1.0 :`A` 1.0))
        (else
          (`KismetSystemLibrary.PrintString` "Line of sight is clear!" true true (struct :`G` 1.0 :`A` 1.0))))
      (else
        (`KismetSystemLibrary.PrintString` "No target selected in details panel" true true (struct :`R` 1.0 :`A` 1.0))))))

(fn `UserConstructionScript`
  (bind _eyeline (`self.Eyeline`))
  (bind (_returnvalue_x _returnvalue_y _returnvalue_z) (`KismetMathLibrary.BreakVector` (`SceneComponent.K2_GetComponentLocation` _eyeline)))
  (`SceneComponent.K2_SetWorldLocation` _eyeline (`KismetMathLibrary.MakeVector` _returnvalue_x _returnvalue_y (+ _returnvalue_z (`self.Offset`))) false false)
  (if (`self.ShowMesh?`)
    (`SkinnedMeshComponent.SetSkinnedAssetAndUpdate` (`self.SkeletalMesh`) (`self.Skele Mesh`) true)
    (`SceneComponent.SetVisibility` (`self.SkeletalMesh`) true false)
    (`SceneComponent.SetVisibility` (`self.Capsule`) false false)
    (else
      (`SceneComponent.SetVisibility` (`self.Capsule`) true false)
      (`SceneComponent.SetVisibility` (`self.SkeletalMesh`) false false))))