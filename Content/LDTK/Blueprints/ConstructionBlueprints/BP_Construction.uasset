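; BP_Construction is a modular building actor that tiles a static mesh in a straight line along one chosen axis.
; Its construction script divides the EndPoint distance by the piece Length and spawns that many mesh components, each offset along the axis with a shared Rotation and Material.
; While tiling, it also constrains EndPoint to that axis and sets the actor's Tags to a single configurable Tag.
; The event graph is unused.
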(fn `UserConstructionScript`
  (bind _length (`self.Length`))
  (bind (_endpoint_x _endpoint_y _endpoint_z) (`KismetMathLibrary.BreakVector` (`self.EndPoint`)))
  (bind _returnvalue (- (* (`self.LastIndex`) _length) _length))
  (if (!= (* (`self.EndPoint`) (1.0 1.0 1.0)) (0.0 0.0 0.0))
    (for _index (range 1 (+ (`KismetMathLibrary.FFloor` (/ (`KismetMathLibrary.VSize` (`self.EndPoint`)) (`self.Length`))) 1))
      (set `self.LastIndex` _index)
      (bind _returnvalue_2 (`AddComponent|NODE_AddStaticMeshComponent-0` :`RelativeTransform` (`KismetMathLibrary.MakeTransform` (0.0 0.0 0.0) (`self.Rotation`))))
      (`StaticMeshComponent.SetStaticMesh` _returnvalue_2 (`self.Mesh`))
      (`PrimitiveComponent.SetMaterial` _returnvalue_2 0 (`self.Material`))
      (`SceneComponent.K2_AttachToComponent` _returnvalue_2 (`self.DefaultSceneRoot`) "None" "KeepWorld" "KeepWorld" "KeepWorld" true)
      (`SceneComponent.K2_SetRelativeLocationAndRotation` _returnvalue_2 (select `/Game/LDTK/Blueprints/Enums/XYZ_Enum` (`self.XYZ`) :`NewEnumerator0` (`KismetMathLibrary.MakeVector` _returnvalue) :`NewEnumerator1` (`KismetMathLibrary.MakeVector` 0.0 _returnvalue) :`NewEnumerator3` (`KismetMathLibrary.MakeVector` 0.0 0.0 _returnvalue) :!type "Vector Structure") (`self.Rotation`) false false)
      (set `self.Tags` (`|MakeArray` (`self.Tag`)))
      (set `self.EndPoint` (select `/Game/LDTK/Blueprints/Enums/XYZ_Enum` (`self.XYZ`) :`NewEnumerator0` (`KismetMathLibrary.MakeVector` _endpoint_x) :`NewEnumerator1` (`KismetMathLibrary.MakeVector` 0.0 _endpoint_y) :`NewEnumerator3` (`KismetMathLibrary.MakeVector` 0.0 0.0 _endpoint_z) :!type "Vector Structure")))))