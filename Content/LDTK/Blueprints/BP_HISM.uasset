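; BP_HISM merges all actors sharing a tag into one hierarchical instanced static mesh using a set mesh and material.
; Convert moves itself to the world origin, adds an instance at each tagged actor's transform, then destroys those actors.
; BeginPlay runs the same conversion unless Convert has already set the Converted flag.
; Revert spawns a StaticMeshActor per instance, clears the instances and destroys itself.
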(event `Convert`
  (bind _hism (`self.HISM`))
  (set `self.Converted?` true)
  (`self.K2_SetActorLocation` (0.0 0.0 0.0) :!label _label)
  (`StaticMeshComponent.SetStaticMesh` (`self.HISM`) (`self.Mesh`))
  (bind _outactors (`GameplayStatics.GetAllActorsWithTag` (`KismetStringLibrary.Conv_StringToName` (`self.Tag`))))
  (for _array_element _outactors
    (`KismetArrayLibrary.Array_Add` (`self.MeshArray`) _array_element)
    (`KismetArrayLibrary.Array_Add` (`self.MeshTransform`) (`self.GetTransform` _array_element)))
  (for _array_element_2 (`self.MeshTransform`)
    (`InstancedStaticMeshComponent.AddInstance` _hism _array_element_2)
    (`PrimitiveComponent.SetMaterial` _hism 0 (`self.Material`)))
  (for _array_element_3 (`self.MeshArray`)
    (if (`KismetSystemLibrary.IsValid` _array_element_3)
      (`self.K2_DestroyActor` _array_element_3))))

(event `self.ReceiveBeginPlay`
  (if (not (`self.Converted?`))
    (goto _label)))

(event `Revert`
  (bind _hism (`self.HISM`))
  (for _index (range (`InstancedStaticMeshComponent.GetInstanceCount` _hism))
    (bind _returnvalue (`|SpawnActorFromClass` "/Script/Engine.StaticMeshActor" (`InstancedStaticMeshComponent.GetInstanceTransform` _hism _index true) "Undefined" "OverrideRootScale" null null))
    (bind _staticmeshcomponent (`StaticMeshActor.StaticMeshComponent` _returnvalue))
    (`StaticMeshComponent.SetStaticMesh` _staticmeshcomponent (`self.Mesh`))
    (`PrimitiveComponent.SetMaterial` _staticmeshcomponent 0 (`self.Material`)))
  (`InstancedStaticMeshComponent.ClearInstances` _hism)
  (`self.K2_DestroyActor`))

(fn `UserConstructionScript`)